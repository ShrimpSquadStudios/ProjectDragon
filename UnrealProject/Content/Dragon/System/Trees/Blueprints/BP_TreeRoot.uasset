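; BP_TreeRoot is a tree root actor that grows a chain of copies of itself across the ground plane.
; One second after BeginPlay, if RootBeside is false, it spawns another root 25 units away in a random direction with matching yaw, then sets the flag.
; Each copy runs the same logic, with no depth limit or occupancy check.
; RandomInteger(3) yields 0 to 2, so AddRootDown is never reached.
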(event `self.ReceiveBeginPlay`
  (`KismetSystemLibrary.Delay` 1.0)
  (if (not (`self.RootBeside`))
    (switch `int` (`KismetMathLibrary.RandomInteger` 3)
      (:`Default`
        (`self.AddRootLeft` :!label _label))
      (:`0`
        (goto _label))
      (:`1`
        (`self.AddRootRight`))
      (:`2`
        (`self.AddRootUp`))
      (:`3`
        (`self.AddRootDown`)))
    (set `self.RootBeside` true)))

(event `self.ReceiveTick`
  (params (DeltaSeconds :type "Float (single-precision)")))

(fn `AddRootDown`
  (bind _returnvalue (`self.GetTransform`))
  (`|SpawnActorFromClass` "BP_TreeRoot_C" (`KismetMathLibrary.MakeTransform` (`KismetMathLibrary.MakeVector` (+ -25.0 (.x (.location _returnvalue))) (.y (.location _returnvalue)) (.z (.location _returnvalue))) (`KismetMathLibrary.MakeRotator` (.roll (.rotation _returnvalue)) (.pitch (.rotation _returnvalue)) -90.0) (.scale _returnvalue)) "Undefined" "MultiplyWithRoot" null 0 null))

(fn `AddRootLeft`
  (bind _returnvalue (`self.GetTransform`))
  (`|SpawnActorFromClass` "BP_TreeRoot_C" (`KismetMathLibrary.MakeTransform` (`KismetMathLibrary.MakeVector` (.x (.location _returnvalue)) (+ -25.0 (.y (.location _returnvalue))) (.z (.location _returnvalue))) (`KismetMathLibrary.MakeRotator` (.roll (.rotation _returnvalue)) (.pitch (.rotation _returnvalue)) 180.0) (.scale _returnvalue)) "Undefined" "MultiplyWithRoot" null 0 null))

(fn `AddRootRight`
  (bind _returnvalue (`self.GetTransform`))
  (`|SpawnActorFromClass` "BP_TreeRoot_C" (`KismetMathLibrary.MakeTransform` (`KismetMathLibrary.MakeVector` (.x (.location _returnvalue)) (+ 25.0 (.y (.location _returnvalue))) (.z (.location _returnvalue))) (`KismetMathLibrary.MakeRotator` (.roll (.rotation _returnvalue)) (.pitch (.rotation _returnvalue))) (.scale _returnvalue)) "Undefined" "MultiplyWithRoot" null 0 null))

(fn `AddRootUp`
  (bind _returnvalue (`self.GetTransform`))
  (`|SpawnActorFromClass` "BP_TreeRoot_C" (`KismetMathLibrary.MakeTransform` (`KismetMathLibrary.MakeVector` (+ (.x (.location _returnvalue)) 25.0) (.y (.location _returnvalue)) (.z (.location _returnvalue))) (`KismetMathLibrary.MakeRotator` (.roll (.rotation _returnvalue)) (.pitch (.rotation _returnvalue)) 90.0) (.scale _returnvalue)) "Undefined" "MultiplyWithRoot" null 0 null))

(fn `UserConstructionScript`)