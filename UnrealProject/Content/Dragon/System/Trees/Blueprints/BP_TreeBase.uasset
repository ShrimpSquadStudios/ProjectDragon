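; BP_TreeBase is a tree actor that grows from root segments, using sunlight as its growth resource.
; On BeginPlay it spawns a half-scale BP_TreeRoot at its location and tracks it as the current root.
; Each Tick with at least one sunlight in its sunlight component, it asks the current root to build the next one.
; On success the new root becomes current and one sunlight is spent.
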(event `self.ReceiveBeginPlay`
  (bind _returnvalue (`|SpawnActorFromClass` "/Game/Dragon/System/Trees/Blueprints/BP_TreeRoot.BP_TreeRoot_C" (`KismetMathLibrary.MakeTransform` (`self.K2_GetActorLocation`) (struct) (0.5 0.5 0.5)) "Undefined" "MultiplyWithRoot" null 0 null))
  (set `self.CurrentTreeRoot` _returnvalue))

(event `self.ReceiveTick`
  (params (DeltaSeconds :type "Float (single-precision)"))
  (bind _sunlight (`/Game/Dragon/System/Resources/BP_SunlightComponent.Get Sunlight Amount` (`/Game/Dragon/Core/BPFL_Components.GetSunlightComponent`)))
  (`/Engine/EditorBlueprintResources/StandardMacros.CompareInt` _sunlight 1
    (:`>`
      _)
    (:`==`
      _))
  (bind (_success _nexttreeroot) (`/Game/Dragon/System/Trees/Blueprints/BP_TreeRoot.BuildNextRoot` (`self.CurrentTreeRoot`)))
  (if _success
    (set `self.CurrentTreeRoot` _nexttreeroot)
    (`/Game/Dragon/System/Resources/BP_SunlightComponent.Add to Sunlight Amount` (`/Game/Dragon/Core/BPFL_Components.GetSunlightComponent`) -1)))

(fn `UserConstructionScript`)