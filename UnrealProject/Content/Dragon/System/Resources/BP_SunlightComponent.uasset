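; BP_SunlightComponent is a resource component that accumulates a Sunlight value during the daytime.
; Each Tick it reads the Day flag from BPDayNightComponent on BP_GameState and, if set, adds one to Sunlight, so the gain depends on frame rate.
; It also prints the current total on screen every frame as a debug readout.
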(event `self.ReceiveTick`
  (params (DeltaSeconds :type "Float (single-precision)"))
  (`KismetSystemLibrary.PrintString` (`KismetStringLibrary.Concat_StrStr` "Sunlight: " (`KismetStringLibrary.Conv_IntToString` (`self.Sunlight`))) true false (struct :`G` 0.66 :`B` 1.0 :`A` 1.0) DeltaSeconds)
  (bind _asbp_game_state (cast `/Game/Dragon/Core/BP_GameState` (`GameplayStatics.GetGameState`)))
  (if (`/Game/Dragon/System/DayNightCycle/BP_DayNightComponent.Day` (`/Game/Dragon/Core/BP_GameState.BP_DayNightComponent` _asbp_game_state))
    (set `self.Sunlight` (+ (`self.Sunlight`) 1))))