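; Component that holds a Phosphorous resource count, with functions to get, set, add to and subtract from it.
; Every Tick it searches for all BP_ResourceNode_Phosphorous actors and adds one for each whose RootOverlapping flag is set, so the gain rate depends on frame rate.
; Subtraction applies only when the result stays at zero or above, returning whether it succeeded.
; Each gain also prints a debug message.
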(event `self.ReceiveTick`
  (params (DeltaSeconds :type "Float (single-precision)"))
  (bind _outactors (`GameplayStatics.GetAllActorsOfClass` "/Game/Dragon/System/Resources/BP_ResourceNode_Phosphorous.BP_ResourceNode_Phosphorous_C"))
  (for _array_element _outactors
    (if (`/Game/Dragon/System/Resources/BP_ResourceNode_Phosphorous.RootOverlapping` _array_element)
      (`/Game/Dragon/System/Resources/BPFL_Resources.AddPhosphorousAmount` 1)
      (`KismetSystemLibrary.PrintString` "Phosphorous Added"))))

(fn `Add to Phosphorous Amount`
  (params (`Amount To Add` :type Integer))
  (bind _phosphorous (`self.Get Phosphorous Amount`))
  (set `self.Phosphorous` (+ _phosphorous `Amount To Add`)))

(fn `Get Phosphorous Amount`
  (returns (Phosphorous :type Integer))
  (return (`self.Phosphorous`)))

(fn `Set Phosphorous Amount`
  (params (`New Amount` :type Integer))
  (set `self.Phosphorous` `New Amount`))

(fn `Subtract to Phosphorous Amount`
  (params (`Amount to Subtract` :type Integer))
  (returns (Subtracted :type Boolean))
  (bind _phosphorous (`self.Get Phosphorous Amount`))
  (bind _returnvalue (- _phosphorous `Amount to Subtract`))
  (`/Engine/EditorBlueprintResources/StandardMacros.CompareInt` _returnvalue
    (:`>`
      _)
    (:`==`
      _)
    (:`<`
      (return false)))
  (set `self.Phosphorous` _returnvalue)
  (return true))