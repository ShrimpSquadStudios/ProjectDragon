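; Day/night cycle component that rotates the level's directional light to simulate the sun moving.
; BeginPlay caches the first DirectionalLight tagged DayLight.
; Tick pitches it by CycleSpeed scaled by delta time, checking for the two horizon rotations within a tolerance to set the Day flag and switch between day and night speeds.
; Paired DoOnce gates reset each other so each transition fires once per cycle.
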(event `self.ReceiveBeginPlay`
  ;[1 1 1] Get the DayLight from the level through tags
  (bind _outactors (`GameplayStatics.GetAllActorsOfClassWithTag` "/Script/Engine.DirectionalLight" "DayLight"))
  (for _array_element _outactors
    (set `self.DayLight` _array_element)
    (break)))

(event `self.ReceiveTick`
  (params (DeltaSeconds :type "Float (single-precision)"))
  (bind _returnvalue (`Actor.K2_GetActorRotation` (`self.DayLight`)))
  (`Actor.K2_AddActorLocalRotation` (`self.DayLight`) (`KismetMathLibrary.MakeRotator` 0.0 (* DeltaSeconds (`self.CycleSpeed`))) false false)
  (if (== _returnvalue (struct :`Yaw` 180.0 :`Roll` 180.0) :`ErrorTolerance` 1.0)
    (`/Engine/EditorBlueprintResources/StandardMacros.DoOnce` false :!label _label
      (:`Completed`
        (`|ExecutionSequence`
          (:`then_0`
            (set `self.Day` true)
            (set `self.CycleSpeed` (`self.DayCycleSpeed`)))
          (:`then_1`
            (goto _label_2 :!via `Reset`)))))
    (elif (== _returnvalue (struct) :`ErrorTolerance` 1.0)
      (`/Engine/EditorBlueprintResources/StandardMacros.DoOnce` false :!label _label_2
        (:`Completed`
          (`|ExecutionSequence`
            (:`then_0`
              (set `self.Day` false)
              (set `self.CycleSpeed` (`self.NightCycleSpeed`)))
            (:`then_1`
              (goto _label :!via `Reset`))))))))