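; World event component that spawns a wind storm event actor in the world after a random delay.
; A timer start, intended for BeginPlay, arms a one-shot timer with a random delay in seconds and prints a separately rolled value, which can differ from the real delay.
; When the timer fires, it spawns BP_WorldEvent_WindStorm at the world origin; nothing here re-arms the timer afterwards.
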(event `self.ReceiveBeginPlay`
  (`self.Start World Event Timer`))

(event `Start World Event Timer`
  (bind _returnvalue (`KismetMathLibrary.RandomIntegerInRange` 30 120))
  (`KismetSystemLibrary.K2_ClearAndInvalidateTimerHandle` (`self.Timer Handle`))
  (bind _returnvalue_2 (`KismetSystemLibrary.K2_SetTimerDelegate` (delegate `Activate World Event`) (`KismetMathLibrary.Conv_IntToDouble` _returnvalue)))
  (set `self.Timer Handle` _returnvalue_2)
  (`KismetSystemLibrary.PrintString` (`KismetStringLibrary.Concat_StrStr` "World event timer set for: " (`KismetStringLibrary.Conv_IntToString` _returnvalue) " seconds")))

(event `Activate World Event`
  (`self.Start World Event`))

(fn `Start World Event`
  (`|SpawnActorFromClass` "/Game/Dragon/System/WorldEvents/Blueprints/BP_WorldEvent_WindStorm.BP_WorldEvent_WindStorm_C" (`KismetMathLibrary.MakeTransform` (0.0 0.0 0.0)) "Undefined" "MultiplyWithRoot" null null))