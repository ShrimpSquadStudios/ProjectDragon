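; BP_WorldEvent_SnowStorm is a timed snowstorm world event that announces a blizzard and spawns snow VFX.
; WorldEventStart spawns the Niagara system at a fixed location and sets a timer for the event duration, which BeginPlay sets.
; When the timer fires, WorldEventOver sets wind intensity in a material parameter collection, removes the VFX, restarts the GameState's world event timer, and destroys the actor.
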(event `self.ReceiveBeginPlay`
  (`parent.ReceiveBeginPlay`)
  (set `self.World Event Duration` 120.0))

(event `self.ReceiveActorBeginOverlap`
  (params (OtherActor :type "Actor Object Reference"))
  (`parent.ReceiveActorBeginOverlap` OtherActor))

(event `self.World Event Start`
  (`KismetSystemLibrary.K2_ClearAndInvalidateTimerHandle` (`self.Timer Handle`))
  (bind _returnvalue (`KismetSystemLibrary.K2_SetTimerDelegate` (delegate `WorldEventOver`) (`self.World Event Duration`)))
  (set `self.Timer Handle` _returnvalue)
  (bind _returnvalue_2 (`NiagaraFunctionLibrary.SpawnSystemAtLocation` "/Game/Dragon/System/Weather/Snow_VFX.Snow_VFX" (-100.0 -100.0 -100.0)))
  (set `self.SnowVFX` _returnvalue_2)
  (`KismetSystemLibrary.PrintString` "A blizzard is active!" true true (struct :`G` 0.66 :`B` 1.0 :`A` 1.0) (`self.World Event Duration`)))

(event `WorldEventOver`
  (`KismetMaterialLibrary.SetScalarParameterValue` "/Game/Dragon/System/Weather/WindBasic.WindBasic" "W_INTENSITY" 4.0)
  (`KismetSystemLibrary.PrintString` "The snow has stopped" true true (struct :`G` 0.66 :`B` 1.0 :`A` 1.0) 5.0)
  (`ActorComponent.K2_DestroyComponent` (`self.SnowVFX`))
  (bind _asbp_game_state (cast `/Game/Dragon/Core/BP_GameState` (`GameplayStatics.GetGameState`)))
  ;[1 0 0] TODO CONVERT THIS TO DELEGATE
  (`/Game/Dragon/System/WorldEvents/Blueprints/BP_WorldEventComponent.Start World Event Timer` (`/Game/Dragon/Core/BP_GameState.BP_WorldEventComponent` _asbp_game_state))
  (`self.K2_DestroyActor`))

(fn `UserConstructionScript`
  (`parent.UserConstructionScript`))