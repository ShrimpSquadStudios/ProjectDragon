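; BP_WorldEvent_WindStorm is a timed world event that runs a wind storm with rain.
; On start it raises wind intensity in the WindBasic parameter collection, spawns rain Niagara VFX, shows a HUD message and starts a duration timer.
; Tick ramps puddle accumulation from the timer's elapsed time, capped at one.
; The end event resets wind and puddles, removes the rain, restarts the GameState's world event timer and destroys the actor.
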(event `self.ReceiveBeginPlay`
  (`parent.ReceiveBeginPlay`))

(event `self.ReceiveTick`
  (params (DeltaSeconds :type "Float (single-precision)"))
  (`parent.ReceiveTick` DeltaSeconds)
  (`KismetMaterialLibrary.SetScalarParameterValue` "/Game/Dragon/System/Weather/WindBasic.WindBasic" "PUDDLE_ACCUMULATION" (`KismetMathLibrary.FMin` (/ (`KismetSystemLibrary.K2_GetTimerElapsedTimeHandle` (`self.TimerHandle`)) 100.0) 1.0)))

(event `self.World Event Start`
  (`/Game/Dragon/UI/HUD/BP_HUDComponent.ShowWorldEvent` (`/Game/Dragon/Core/BPFL_Components.GetHUDComponent`) "A wind storm is active!")
  (`KismetMaterialLibrary.SetScalarParameterValue` "/Game/Dragon/System/Weather/WindBasic.WindBasic" "W_INTENSITY" 20.0)
  (bind _returnvalue (`NiagaraFunctionLibrary.SpawnSystemAtLocation` "/Game/Dragon/System/Weather/Rain_VFX.Rain_VFX" (-100.0 -100.0 -100.0)))
  (set `self.RainVFX` _returnvalue)
  (`KismetSystemLibrary.K2_ClearAndInvalidateTimerHandle` (`self.TimerHandle`))
  (bind _returnvalue_2 (`KismetSystemLibrary.K2_SetTimerDelegate` (delegate `World Event Over`) (`self.WorldEventDuration`)))
  (set `self.TimerHandle` _returnvalue_2))

(event `World Event Over`
  (`KismetMaterialLibrary.SetScalarParameterValue` "/Game/Dragon/System/Weather/WindBasic.WindBasic" "W_INTENSITY" 4.0)
  (`KismetMaterialLibrary.SetScalarParameterValue` "/Game/Dragon/System/Weather/WindBasic.WindBasic" "PUDDLE_ACCUMULATION")
  (`/Game/Dragon/UI/HUD/BP_HUDComponent.ShowWorldEvent` (`/Game/Dragon/Core/BPFL_Components.GetHUDComponent`) "The winds have calmed")
  (bind _asbp_game_state (cast `/Game/Dragon/Core/BP_GameState` (`GameplayStatics.GetGameState`)))
  (`ActorComponent.K2_DestroyComponent` (`self.RainVFX`))
  (`/Game/Dragon/System/WorldEvents/Blueprints/BP_WorldEventComponent.Start World Event Timer` (`/Game/Dragon/Core/BP_GameState.BP_WorldEventComponent` _asbp_game_state))
  (`self.K2_DestroyActor`))

(fn `UserConstructionScript`
  (`parent.UserConstructionScript`))