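; Component that handles building placement, toggling a hidden preview actor and spawning the selected object's actor on input.
; The preview follows GetMouseLocationOnGrid every tick, currently a placeholder returning the player pawn's XY at zero height, always on ground.
; Confirming subtracts each precondition amount as sunlight regardless of resource type, spawning if the last subtraction succeeds.
; Cancel stops active placement; its destroy-hit-actor branch is unreachable with the placeholder.
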(event `self.ReceiveTick`
  (params (DeltaSeconds :type "Float (single-precision)"))
  (`parent.ReceiveTick` DeltaSeconds)
  (`self.UpdatePreviewActorLocation`))

(event `self.ReceiveBeginPlay`
  (`parent.ReceiveBeginPlay`)
  (`self.SpawnPreviewActor`)
  (`self.HidePreviewActor`))

(event `EnhancedInput|/Game/Dragon/Input/IA_PlaceObject`
  (params (ActionValue :type Boolean) (ElapsedSeconds :type "Float (double-precision)") (TriggeredSeconds :type "Float (double-precision)") (InputAction :type "InputAction Object Reference" :default "/Game/Dragon/Input/IA_PlaceObject.IA_PlaceObject"))
  (:`Completed`
    (`self.ConfirmObjectPlacement`)))

(event `EnhancedInput|/Game/Dragon/Input/IA_Cancel`
  (params (ActionValue :type Boolean) (ElapsedSeconds :type "Float (double-precision)") (TriggeredSeconds :type "Float (double-precision)") (InputAction :type "InputAction Object Reference" :default "/Game/Dragon/Input/IA_Cancel.IA_Cancel"))
  (bind (_returnvalue _isonground _hitactor) (`self.GetMouseLocationOnGrid`))
  (:`Triggered`
    (if (`self.bIsPlacementActive`)
      (`self.StopPlacingObject`)
      (`self.HidePreviewActor`)
      (elif (not _isonground)
        (`/Engine/EditorBlueprintResources/StandardMacros.IsValid` _hitactor
          (:`Is Valid`
            (`Actor.K2_DestroyActor` _hitactor)))))))

(fn `ConfirmObjectPlacement`
  (bind (_returnvalue _isonground) (`self.GetMouseLocationOnGrid`))
  (bind (_name _texture _actor _placementprecondition) (break `/Game/Dragon/System/Building/S_BuildObject` (`self.ObjectData`)))
  (if (`KismetSystemLibrary.IsValidClass` _actor)
    (for _array_element _placementprecondition
      (bind _resourcesubtracted (`self.SubtractResourceRequirement` (break `/Game/Dragon/System/Resources/S_ResourceAdjustments` _array_element) (`.Amount_4_49F775F841610D0361EB33A6A72A2371` (break `/Game/Dragon/System/Resources/S_ResourceAdjustments` _array_element)))))
    (if _resourcesubtracted
      (if _isonground
        _
        (else
          _))
      (`|SpawnActorFromClass` (`.Actor_12_93637CED4B750BF23DB7F189A0613667` (break `/Game/Dragon/System/Building/S_BuildObject` (`self.ObjectData`))) (`KismetMathLibrary.MakeTransform` _returnvalue) "Undefined" "MultiplyWithRoot" null null)
      (else
        (`KismetSystemLibrary.PrintString` "Not enough resources to place object")))))

(fn `GetMouseLocationOnGrid`
  (returns (ReturnValue :type "Vector Structure") (IsOnGround :type Boolean) (HitActor :type "Actor Object Reference"))
  (locals (GroundHeight :type "Float (double-precision)" :default 0.0))
  (bind (_returnvalue_x _returnvalue_y) (`KismetMathLibrary.BreakVector` (`Actor.K2_GetActorLocation` (`GameplayStatics.GetPlayerPawn` 0))))
  ;[1 0 0] TODO make this use mouse location
  (return (`KismetMathLibrary.MakeVector` _returnvalue_x _returnvalue_y) true null))

(fn `HidePreviewActor`
  (`Actor.SetActorHiddenInGame` (`self.PreviewActor`) true))

(fn `ShowPreviewActor`
  (`Actor.SetActorHiddenInGame` (`self.PreviewActor`) false))

(fn `SpawnPreviewActor`
  (bind _returnvalue (`|SpawnActorFromClass` "/Game/Dragon/System/Building/BP_PreviewActor.BP_PreviewActor_C" (`KismetMathLibrary.MakeTransform` (0.0 0.0 0.0)) "Undefined" "MultiplyWithRoot" null null))
  (set `self.PreviewActor` _returnvalue))

(fn `StartPlacingObject`
  (params (ObjectData :type "/Game/Dragon/System/Building/S_BuildObject Structure"))
  (set `self.ObjectData` ObjectData)
  (`self.ShowPreviewActor`)
  (set `self.bIsPlacementActive` true))

(fn `StopPlacingObject`
  (set `self.ObjectData` (struct))
  (`self.HidePreviewActor`)
  (set `self.bIsPlacementActive` false))

(fn `SubtractResourceRequirement`
  (params (Resource :type "/Game/Dragon/System/Resources/Enum_ResourceTypes Enum" :default "NewEnumerator0") (Amount :type Integer))
  (returns (ResourceSubtracted :type Boolean))
  (bind _success (`/Game/Dragon/System/Resources/BPFL_Resources.SubtractSunlightAmount` Amount))
  (return _success))

(fn `UpdatePreviewActorLocation`
  (bind _previewactor (`self.PreviewActor`)
    (:`then`
      (`Actor.K2_SetActorLocation` _previewactor (`self.GetMouseLocationOnGrid`) false true))
    (:`else`)))