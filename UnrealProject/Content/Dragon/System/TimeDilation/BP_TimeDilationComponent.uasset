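; BP_TimeDilationComponent is a component that controls game speed, with a paused state and four selectable speeds.
; SetGameSpeed stores the previous and current speed, then either pauses the game or unpauses it and applies global time dilation from a speed-to-factor lookup.
; Each change broadcasts the new speed and dilation factor, and ResumePreviousSpeed restores the last setting.
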(fn `GetFactorFromSpeed`
  (params (Speed :type "/Game/Dragon/System/TimeDilation/E_GameSpeed Enum" :default "NewEnumerator0"))
  (returns (ReturnValue :type "Float (double-precision)"))
  (switch `/Game/Dragon/System/TimeDilation/E_GameSpeed` Speed
    (:`NewEnumerator0`
      (return 0.0))
    (:`NewEnumerator1`
      (return 1.0))
    (:`NewEnumerator2`
      (return 3.0))
    (:`NewEnumerator3`
      (return 5.0))
    (:`NewEnumerator4`
      (return 10.0))))

(fn `GetGameSpeed`
  (returns (CurrentGameSpeed :type "/Game/Dragon/System/TimeDilation/E_GameSpeed Enum"))
  (return (`self.CurrentGameSpeed`)))

(fn `GetTimeDilationFactor`
  (returns (ReturnValue :type "Float (double-precision)"))
  (return (`self.CurrentTimeDilation`)))

(fn `IsGamePaused`
  (returns (ReturnValue :type Boolean))
  (return (`self.bIsGamePaused`)))

(fn `ResumePreviousSpeed`
  (`self.SetGameSpeed` (`self.PreviousGameSpeed`)))

(fn `SetGameSpeed`
  (params (Speed :type "/Game/Dragon/System/TimeDilation/E_GameSpeed Enum" :default "NewEnumerator0"))
  (set `self.PreviousGameSpeed` (`self.CurrentGameSpeed`))
  (set `self.CurrentGameSpeed` (`local.Speed`))
  (set `self.bIsGamePaused` (`|EnumEquality` (`local.Speed`) "NewEnumerator0"))
  (switch `/Game/Dragon/System/TimeDilation/E_GameSpeed` (`local.Speed`)
    (:`NewEnumerator0`
      (`GameplayStatics.SetGamePaused` true))
    (:`NewEnumerator1`
      (`GameplayStatics.SetGamePaused` false :!label _label)
      (bind _output_get (set `self.CurrentTimeDilation` (`self.GetFactorFromSpeed` (`local.Speed`))))
      (`GameplayStatics.SetGlobalTimeDilation` _output_get))
    (:`NewEnumerator2`
      (goto _label))
    (:`NewEnumerator3`
      (goto _label))
    (:`NewEnumerator4`
      (goto _label)))
  (`self.OnGameSpeedChanged` (`local.Speed`) (`self.CurrentTimeDilation`)))