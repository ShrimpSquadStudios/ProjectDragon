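; Player controller that pans the top-down view in response to four directional camera input actions.
; While an action is ongoing, its matching function casts the player pawn to BP_TopDownCharacter and sets a new location offset by CameraSpeed.
; Up and down shift along world X and left and right along world Y, moving the pawn itself with no delta-time scaling.
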(event `EnhancedInput|/Game/Dragon/Input/IA_CameraUp`
  (params (ActionValue :type Boolean) (ElapsedSeconds :type "Float (double-precision)") (TriggeredSeconds :type "Float (double-precision)") (InputAction :type "InputAction Object Reference" :default "/Game/Dragon/Input/IA_CameraUp.IA_CameraUp"))
  (:`Ongoing`
    (`self.MoveCameraUp`)))

(event `EnhancedInput|/Game/Dragon/Input/IA_CameraDown`
  (params (ActionValue :type Boolean) (ElapsedSeconds :type "Float (double-precision)") (TriggeredSeconds :type "Float (double-precision)") (InputAction :type "InputAction Object Reference" :default "/Game/Dragon/Input/IA_CameraDown.IA_CameraDown"))
  (:`Ongoing`
    (`self.MoveCameraDown`)))

(event `EnhancedInput|/Game/Dragon/Input/IA_CameraLeft`
  (params (ActionValue :type Boolean) (ElapsedSeconds :type "Float (double-precision)") (TriggeredSeconds :type "Float (double-precision)") (InputAction :type "InputAction Object Reference" :default "/Game/Dragon/Input/IA_CameraLeft.IA_CameraLeft"))
  (:`Ongoing`
    (`self.MoveCameraLeft`)))

(event `EnhancedInput|/Game/Dragon/Input/IA_CameraRight`
  (params (ActionValue :type Boolean) (ElapsedSeconds :type "Float (double-precision)") (TriggeredSeconds :type "Float (double-precision)") (InputAction :type "InputAction Object Reference" :default "/Game/Dragon/Input/IA_CameraRight.IA_CameraRight"))
  (:`Ongoing`
    (`self.MoveCameraRight`)))

(fn `MoveCameraDown`
  (bind _asbp_top_down_character (cast `/Game/TopDown/Blueprints/BP_TopDownCharacter` (`GameplayStatics.GetPlayerPawn` 0)))
  (bind (_returnvalue_x _returnvalue_y _returnvalue_z) (`KismetMathLibrary.BreakVector` (`self.K2_GetActorLocation` _asbp_top_down_character)))
  (`self.K2_SetActorLocation` _asbp_top_down_character (`KismetMathLibrary.MakeVector` (- _returnvalue_x (`self.CameraSpeed`)) _returnvalue_y _returnvalue_z) false false))

(fn `MoveCameraLeft`
  (bind _asbp_top_down_character (cast `/Game/TopDown/Blueprints/BP_TopDownCharacter` (`GameplayStatics.GetPlayerPawn` 0)))
  (bind (_returnvalue_x _returnvalue_y _returnvalue_z) (`KismetMathLibrary.BreakVector` (`self.K2_GetActorLocation` _asbp_top_down_character)))
  (`self.K2_SetActorLocation` _asbp_top_down_character (`KismetMathLibrary.MakeVector` _returnvalue_x (- _returnvalue_y (`self.CameraSpeed`)) _returnvalue_z) false false))

(fn `MoveCameraRight`
  (bind _asbp_top_down_character (cast `/Game/TopDown/Blueprints/BP_TopDownCharacter` (`GameplayStatics.GetPlayerPawn` 0)))
  (bind (_returnvalue_x _returnvalue_y _returnvalue_z) (`KismetMathLibrary.BreakVector` (`self.K2_GetActorLocation` _asbp_top_down_character)))
  (`self.K2_SetActorLocation` _asbp_top_down_character (`KismetMathLibrary.MakeVector` _returnvalue_x (+ _returnvalue_y (`self.CameraSpeed`)) _returnvalue_z) false false))

(fn `MoveCameraUp`
  (bind _asbp_top_down_character (cast `/Game/TopDown/Blueprints/BP_TopDownCharacter` (`GameplayStatics.GetPlayerPawn` 0)))
  (bind (_returnvalue_x _returnvalue_y _returnvalue_z) (`KismetMathLibrary.BreakVector` (`self.K2_GetActorLocation` _asbp_top_down_character)))
  (`self.K2_SetActorLocation` _asbp_top_down_character (`KismetMathLibrary.MakeVector` (+ _returnvalue_x (`self.CameraSpeed`)) _returnvalue_y _returnvalue_z) false false))

(fn `UserConstructionScript`)